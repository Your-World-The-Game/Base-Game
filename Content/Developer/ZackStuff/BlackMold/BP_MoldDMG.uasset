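; BP_MoldDMG is a black mold hazard that slows and damages the first-person player while inside its collision.
; On overlap it halves walk speed, disables sprint and starts a looping one-second timer that drains the player's health component.
; The health component's Dead event is bound to restart the level.
; Shortly after exit it clears the timer, restores movement, resets player damage states and calls HealPlayer.
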(event OnComponentBeginOverlap(Collision)
  (params (OverlappedComponent :type Primitive%20Component%20Object%20Reference) (OtherActor :type Actor%20Object%20Reference) (OtherComp :type Primitive%20Component%20Object%20Reference) (OtherBodyIndex :type Integer) (bFromSweep :type Boolean) (SweepResult :type Hit%20Result%20Structure%20%28by%20ref%29))
  ;[0.15 0.15 0.15 0.5] Collision Mold ON
  (bind _asbp_test_first_person (Utilities|Casting|CastToBP_TestFirstPerson OtherActor))
  (bind _output_get (Variables|Default|SetPlayer%20Reference _asbp_test_first_person))
  (Utilities|FlowControl|Sequence
    (:then_0
      (CallFunction|SlowPlayer)
      (Development|PrintString "You've been slowed"))
    (:then_1
      (bind _returnvalue (Utilities|Time|SetTimerbyEvent (delegate Custom|Drain%20Health) 1.0 true))
      (EventDispatchers|BindEventtoDead (Variables|/Game/Developer/ZackStuff/Blueprints/BP_TestFirstPerson.BP_TestFirstPerson_C|GetBPC_Health _output_get) (delegate Custom|Dead)))))

(event OnComponentEndOverlap(Collision)
  (params (OverlappedComponent :type Primitive%20Component%20Object%20Reference) (OtherActor :type Actor%20Object%20Reference) (OtherComp :type Primitive%20Component%20Object%20Reference) (OtherBodyIndex :type Integer))
  (bind _player_reference (Variables|Default|GetPlayer%20Reference))
  ;[0.15 0.15 0.15 0.5] Collision Mold OFF
  (Utilities|Casting|CastToBP_TestFirstPerson OtherActor)
  (Utilities|FlowControl|Delay 0.2)
  (Utilities|FlowControl|Sequence
    (:then_0
      (Utilities|Time|ClearandInvalidateTimerbyHandle (stale OnComponentBeginOverlap(Collision) _returnvalue)))
    (:then_1
      (CallFunction|RestoreSpeed))
    (:then_2
      (Default|PlayerIsNoLongerGettingDamaged _player_reference))
    (:then_3
      (Default|HealPlayer _player_reference))
    (:then_4
      (Default|PlayerIsNoLongeronMold _player_reference))))

(event Custom|Drain%20Health
  (bind _player_reference (Variables|Default|GetPlayer%20Reference))
  (bind _bpc_health (Variables|/Game/Developer/ZackStuff/Blueprints/BP_TestFirstPerson.BP_TestFirstPerson_C|GetBPC_Health _player_reference))
  ;[0.15 0.15 0.15 0.5] Drain Player's Health Per Second in Mold
  (Default|PlayerIsonMold _player_reference)
  (Default|PlayerIsGettingDamaged _player_reference)
  (Default|HealthDecrease _bpc_health 1e+01)
  (Development|PrintString (Utilities|String|ToString(Float) (Variables|/Game/Developer/ZackStuff/Blueprints/BPC_Health.BPC_Health_C|GetHealth _bpc_health))))

(event Custom|Slow%20Player
  (bind _player_reference (Variables|Default|GetPlayer%20Reference))
  ;[0.15 0.15 0.15 0.5] Slow the Player
  (Variables|/Script/Engine.CharacterMovementComponent|SetMaxWalkSpeed (Variables|/Script/Engine.Character|GetCharacterMovement _player_reference) 1.5e+02)
  (Variables|/Game/Developer/ZackStuff/Blueprints/BP_TestFirstPerson.BP_TestFirstPerson_C|SetbCanPlayerSprint? _player_reference false))

(event Custom|Dead
  ;[0.15 0.15 0.15 0.5] Collision Mold ON
  (Development|ExecuteConsoleCommand "RestartLevel" 0))

(event Custom|Restore%20Speed
  (bind _player_reference (Variables|Default|GetPlayer%20Reference))
  ;[0.15 0.15 0.15 0.5] Restore Speed to Player
  (Variables|/Script/Engine.CharacterMovementComponent|SetMaxWalkSpeed (Variables|/Script/Engine.Character|GetCharacterMovement _player_reference) 3e+02)
  (Variables|/Game/Developer/ZackStuff/Blueprints/BP_TestFirstPerson.BP_TestFirstPerson_C|SetbCanPlayerSprint? _player_reference true))

(fn ConstructionScript)